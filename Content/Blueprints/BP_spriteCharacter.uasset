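; Paper2D player character for a side-view jumping game, moved along the X axis by input and jumping with Space.
; BeginPlay shows the instructions widget and sets the idle flipbook.
; Tick resets the character to a fixed point after a fall, swaps idle and frog-jump flipbooks by speed, and flips facing through control rotation.
; Above a height threshold, Tick also shows the win screen after a short delay, with no one-time guard.
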(event Custom|UpdateAnimation
  (Sprite|SetFlipbook (Variables|Default|GetSprite) (select (> (Math|Vector|VectorLength (Variables|/Script/Engine.MovementComponent|GetVelocity (Variables|Character|GetCharacterMovement))) 0.0) "/Game/SunnyLandAssets/sprites/frog/jumpANimation/FrogJumping.FrogJumping" "/Game/SunnyLandAssets/sprites/frog/FB_Player_Idle.FB_Player_Idle")))

(event Custom|UpdateControlRotation
  (Utilities|IsValid (Pawn|GetController)
    (:Is%20Valid
      (Math|Float|CompareFloat (.X (Math|Vector|BreakVector (Variables|/Script/Engine.MovementComponent|GetVelocity (Variables|Character|GetCharacterMovement)))) 0.0
        (:>
          (Pawn|SetControlRotation (Pawn|GetController) (Math|Rotator|MakeRotator 0.0 0.0 1.8e+02)))
        (:<
          (Pawn|SetControlRotation (Pawn|GetController) (Math|Rotator|MakeRotator 0.0 0.0 0.0)))))))

(event EventBeginPlay
  ;[1 1 1] Widgets werden erstellt und dem Viewport hinzugefügt
  (Utilities|FlowControl|Sequence
    (:then_0
      (bind _returnvalue (UserInterface|CreateWidget "/Game/Blueprints/Instructions.Instructions_C" (Game|GetPlayerController 0)))
      (UserInterface|Viewport|AddtoViewport _returnvalue 0))
    (:then_1
      (Sprite|SetFlipbook (Variables|Default|GetSprite) "/Game/SunnyLandAssets/sprites/frog/FB_Player_Idle.FB_Player_Idle"))))

(event EventTick
  (params (DeltaSeconds :type Float%20%28single-precision%29))
  ;[1 1 1] Spawnpointreset
  (Utilities|FlowControl|Sequence
    (:then_0
      (if (<= (.z (Transformation|GetActorLocation)) -1e+02)
        (Transformation|SetActorLocation "0.000000,0.000000,-57.000000" false false)))
    (:then_1
      (if (>= (.z (Transformation|GetActorLocation)) 2.73e+03)
        (Utilities|FlowControl|Delay 0.5)
        (bind _returnvalue (UserInterface|CreateWidget "/Game/Blueprints/WinScreen.WinScreen_C"))
        (UserInterface|Viewport|AddtoViewport _returnvalue 0)))
    (:then_2
      (CallFunction|UpdateAnimation)
      (CallFunction|UpdateControlRotation))))

(event Input|AxisEvents|InputAxisMovePlayer
  (params (AxisValue :type Float%20%28single-precision%29))
  ;[1 1 1] Mit Arrows  Character nach links/rechts steuern
  (Pawn|Input|AddMovementInput "1.000000,0.000000,0.000000" AxisValue false))

(event Input|KeyboardEvents|SpaceBar
  (params (Key :type Key%20Structure :default "None"))
  (:Pressed
    (Character|Jump)))

(fn ConstructionScript)